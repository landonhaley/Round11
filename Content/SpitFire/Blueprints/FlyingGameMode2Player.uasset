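; Game mode for the SpitFire flying game that spawns and possesses a flyer for the local player on BeginPlay.
; ChoosePlayerStart picks the first PlayerStart not tagged "Taken" and tags it, giving the spawn transform for a CurrentFlyer with non-uniform scale.
; Player 1's FlyingController receives its PlayerNum before possessing the flyer.
; Despite the 2Player name, similar spawn chains for players 2 to 4 are disconnected and never run.
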(event `self.ReceiveBeginPlay`
  (bind _returnvalue (`GameplayStatics.GetPlayerController` 0))
  ;[1 1 1] Player 1 Spawn
  (`GameplayStatics.CreatePlayer` 0)
  (bind _selectedplayerstart (`self.choosePlayerStart`))
  (bind (_returnvalue_location _returnvalue_rotation) (`KismetMathLibrary.BreakTransform` (`self.GetTransform` _selectedplayerstart)))
  (bind _output_get (set `self.Player1Spawn` (`KismetMathLibrary.MakeTransform` _returnvalue_location _returnvalue_rotation (1.0 2.0 0.5))))
  (bind _returnvalue_2 (`|SpawnActorFromClass` "/Game/SpitFire/Blueprints/CurrentFlyer.CurrentFlyer_C" _output_get true))
  (bind _asflying_controller (cast `/Game/SpitFire/Blueprints/FlyingController` _returnvalue))
  (set `/Game/SpitFire/Blueprints/FlyingController.PlayerNum` 0 _asflying_controller)
  (`Controller.Possess` _returnvalue _returnvalue_2))

(fn `choosePlayerStart`
  (returns (SelectedPlayerStart :type "PlayerStart Object Reference") (`Found Player Start` :type Boolean))
  (bind _outactors (`GameplayStatics.GetAllActorsOfClass` "/Script/Engine.PlayerStart"))
  (for _array_element _outactors
    (bind _asplayer_start (cast `PlayerStart` _array_element))
    (if (!= (`PlayerStart.PlayerStartTag` _asplayer_start) "Taken")
      (`|ExecutionSequence`
        (:`then_0`
          (break))
        (:`then_1`
          (set `PlayerStart.PlayerStartTag` "Taken" _asplayer_start))
        (:`then_2`
          (return _asplayer_start true))))))

(fn `UserConstructionScript`)